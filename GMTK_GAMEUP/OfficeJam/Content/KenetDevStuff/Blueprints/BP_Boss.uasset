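; Boss actor that receives a BP_Page from the player and completes the "Page" quest.
; A Float timeline started on BeginPlay drives its relative Z position.
; When a page overlaps its Box, a DoOnce gate lets one submission destroy the page, update the quest on BP_FP_Horror, release the player's physics-handle hold and play a voice line.
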(event OnComponentBeginOverlap(Box)
  (params (OverlappedComponent :type Primitive%20Component%20Object%20Reference) (OtherActor :type Actor%20Object%20Reference) (OtherComp :type Primitive%20Component%20Object%20Reference) (OtherBodyIndex :type Integer) (bFromSweep :type Boolean) (SweepResult :type Hit%20Result%20Structure%20%28by%20ref%29))
  (bind _asbp_page (Utilities|Casting|CastToBP_Page OtherActor))
  (Utilities|FlowControl|DoOnce false
    (:Completed
      (Actor|DestroyActor _asbp_page)
      (bind _asbp_fp_horror (Utilities|Casting|CastToBP_FP_Horror (Game|Player|GetPlayerPawn 0)))
      (Default|CompleteQuest _asbp_fp_horror "Page")
      (Variables|/Game/FirstPerson/Blueprints/BP_FirstPersonCharacter.BP_FirstPersonCharacter_C|SetIsHolding? _asbp_fp_horror false)
      (Physics|Components|PhysicsHandle|ReleaseComponent (Variables|/Game/FirstPerson/Blueprints/BP_FirstPersonCharacter.BP_FirstPersonCharacter_C|GetPhysicsHandle _asbp_fp_horror))
      (Audio|PlaySound2D "/Game/Voiceovers/verbal_VOs/VO_submitdraft.VO_submitdraft" 1.0 1.0 0.0 0 0))))

(event EventTick
  (params (DeltaSeconds :type Float%20%28single-precision%29)))

(event EventBeginPlay
  (bind _newtrack_0 (Timeline|Float Play)
    (:Update
      (Transformation|SetActorRelativeLocation self (Math|Vector|MakeVector 0.0 0.0 (* _newtrack_0 5e+01))))))

(fn ConstructionScript)