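; BP_Toaster is an interactable broken toaster that the player fixes to complete a quest, registered under the name "Projector".
; The first Interact calls CompleteQuest on the BP_FP_Horror pawn, plays the toaster sound, stops BrokenVFX and sets Fixed after a five-second delay.
; An Interact once Fixed is set reactivates BrokenVFX alongside an Explosion effect.
; DoOnce gates limit each stage to a single run.
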(event EventBeginPlay)

(event Collision|EventActorBeginOverlap
  (params (OtherActor :type Actor%20Object%20Reference)))

(event EventTick
  (params (DeltaSeconds :type Float%20%28single-precision%29)))

(event EventInteract
  (if (not (Variables|Default|Getfixed?))
    (Utilities|FlowControl|DoOnce false
      (:Completed
        (bind _asbp_fp_horror (Utilities|Casting|CastToBP_FP_Horror (Game|Player|GetPlayerPawn 0)))
        (Default|CompleteQuest _asbp_fp_horror "Projector")
        (Audio|PlaySound2D "/Game/Sounds/Toaster.Toaster" 1.0 1.0 0.0 0 0)
        (Components|Activation|Deactivate (Variables|Default|GetBrokenVFX))
        (Utilities|FlowControl|Delay 5.0)
        (Variables|Default|Setfixed? true)))
    (else
      (Utilities|FlowControl|DoOnce false
        (:Completed
          (Components|Activation|SetActive (Variables|Default|GetExplosion) true true))))))

(fn ConstructionScript)