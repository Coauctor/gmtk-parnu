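; BP_WaterCooler is the water cooler that completes the "Water" quest when a BP_WaterContainer is brought to it.
; A one-time overlap on its Box component hides the Tank mesh, shows TankComplete and destroys the container.
; It then completes the quest on the BP_FP_Horror player pawn, clears its holding flag and releases its physics handle.
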(event OnComponentBeginOverlap(Box)
  (params (OverlappedComponent :type Primitive%20Component%20Object%20Reference) (OtherActor :type Actor%20Object%20Reference) (OtherComp :type Primitive%20Component%20Object%20Reference) (OtherBodyIndex :type Integer) (bFromSweep :type Boolean) (SweepResult :type Hit%20Result%20Structure%20%28by%20ref%29))
  (bind _asbp_water_container (Utilities|Casting|CastToBP_WaterContainer OtherActor))
  (Utilities|FlowControl|DoOnce false
    (:Completed
      (Rendering|SetVisibility (Variables|Default|GetTank) false false)
      (Rendering|SetVisibility (Variables|Default|GetTankComplete) true false)
      (Actor|DestroyActor _asbp_water_container)
      (bind _asbp_fp_horror (Utilities|Casting|CastToBP_FP_Horror (Game|Player|GetPlayerPawn 0)))
      (Default|CompleteQuest _asbp_fp_horror "Water")
      (Variables|/Game/FirstPerson/Blueprints/BP_FirstPersonCharacter.BP_FirstPersonCharacter_C|SetIsHolding? _asbp_fp_horror false)
      (Physics|Components|PhysicsHandle|ReleaseComponent (Variables|/Game/FirstPerson/Blueprints/BP_FirstPersonCharacter.BP_FirstPersonCharacter_C|GetPhysicsHandle _asbp_fp_horror)))))

(fn ConstructionScript)