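; BP_Worker is an office worker actor that displays character lines when the player character, BP_FP_Horror, overlaps its Box trigger.
; A Box overlap by the player binds a handler to the player's capsule overlap event at that moment, with no unbinding.
; When the capsule's overlapped component is this Box, the handler calls DisplayCharacterLines on the WB_CharacterLine widget held by CharacterLineWidget.
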(event OnComponentBeginOverlap(Box)
  (params (OverlappedComponent :type Primitive%20Component%20Object%20Reference) (OtherActor :type Actor%20Object%20Reference) (OtherComp :type Primitive%20Component%20Object%20Reference) (OtherBodyIndex :type Integer) (bFromSweep :type Boolean) (SweepResult :type Hit%20Result%20Structure%20%28by%20ref%29))
  (bind _asbp_fp_horror (Utilities|Casting|CastToBP_FP_Horror OtherActor))
  (Collision|AssignOnComponentBeginOverlap (Variables|/Script/Engine.Character|GetCapsuleComponent _asbp_fp_horror) (delegate Custom|OnComponentBeginOverlap_Event)))

(event Custom|OnComponentBeginOverlap_Event
  (params (OverlappedComponent :type Primitive%20Component%20Object%20Reference) (OtherActor :type Actor%20Object%20Reference) (OtherComp :type Primitive%20Component%20Object%20Reference) (OtherBodyIndex :type Integer) (bFromSweep :type Boolean) (SweepResult :type Hit%20Result%20Structure%20%28by%20ref%29))
  (if (== OtherComp (Variables|Default|GetBox))
    (bind _aswb_character_line (Utilities|Casting|CastToWB_CharacterLine (UserInterface|GetWidget (Variables|Default|GetCharacterLine_Widget))))
    (Default|DisplayCharacterLines _aswb_character_line)))

(event EventBeginPlay)

(event Collision|EventActorBeginOverlap
  (params (OtherActor :type Actor%20Object%20Reference)))

(event EventTick
  (params (DeltaSeconds :type Float%20%28single-precision%29)))

(fn ConstructionScript)